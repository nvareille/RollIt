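; Roller is a controller Blueprint that rolls a Ball pawn with player input and orbits its camera.
; On BeginPlay it casts the controlled pawn to Ball and caches its Sphere and Camera components.
; Move axes apply torque to the Sphere, rotated by camera yaw so rolling is view-relative.
; LookRight yaws the camera and rotates its world position around the Sphere by the same angle.
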(event `self.ReceiveBeginPlay`
  (bind _asball (cast `/Game/Blueprints/Ball` (`self.K2_GetPawn`)))
  (bind _output_get (set `self.BallVar` _asball))
  (set `self.Sphere` (`/Game/Blueprints/Ball.Sphere` _output_get))
  (set `self.CameraInstance` (`/Game/Blueprints/Ball.Camera` _asball)))

(event `InputAxis|MoveRight`
  (params (AxisValue :type "Float (single-precision)"))
  (`PrimitiveComponent.AddTorque` (`self.Sphere`) (`KismetMathLibrary.RotateAngleAxis` (`KismetMathLibrary.MakeVector` (* AxisValue -10000.0)) (.yaw (`SceneComponent.K2_GetComponentRotation` (`self.CameraInstance`))) (0.0 0.0 1.0)) "None" false))

(event `InputAxis|MoveForward`
  (params (AxisValue :type "Float (single-precision)"))
  (`PrimitiveComponent.AddTorque` (`self.Sphere`) (`KismetMathLibrary.RotateAngleAxis` (`KismetMathLibrary.MakeVector` 0.0 (* AxisValue 10000.0)) (.yaw (`SceneComponent.K2_GetComponentRotation` (`self.CameraInstance`))) (0.0 0.0 1.0)) "None" false))

(event `InputAxis|LookRight`
  (params (AxisValue :type "Float (single-precision)"))
  (bind _returnvalue (* AxisValue 1.0))
  (bind _camerainstance (`self.CameraInstance`))
  (bind _returnvalue_2 (`SceneComponent.K2_GetComponentLocation` (`self.Sphere`)))
  (`SceneComponent.K2_AddWorldRotation` _camerainstance (`KismetMathLibrary.MakeRotator` 0.0 0.0 _returnvalue) false false)
  (`SceneComponent.K2_SetWorldLocation` _camerainstance (+ (`KismetMathLibrary.RotateAngleAxis` (- (`SceneComponent.K2_GetComponentLocation` (`self.CameraInstance`)) _returnvalue_2) _returnvalue (0.0 0.0 1.0)) _returnvalue_2) false false))

(fn `UserConstructionScript`)