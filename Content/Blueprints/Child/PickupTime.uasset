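; Pickup child Blueprint that grants the player extra time.
; It overrides the PickupEffect event to find the top-level HUD widget and add ten to its Time variable.
; The timer value lives on the HUD widget itself, reached through a widget class search rather than a stored reference.
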(event `self.ReceiveBeginPlay`
  (`parent.ReceiveBeginPlay`))

(event `self.ReceiveActorBeginOverlap`
  (params (OtherActor :type "Actor Object Reference")))

(event `self.ReceiveTick`
  (params (DeltaSeconds :type "Float (single-precision)"))
  (`parent.ReceiveTick` 0.0))

(event `self.PickupEffect`
  (bind _foundwidgets (`WidgetBlueprintLibrary.GetAllWidgetsOfClass` "/Game/Blueprints/UI/HUD.HUD_C"))
  (bind _ashud (cast `/Game/Blueprints/UI/HUD` (`KismetArrayLibrary.Array_Get` _foundwidgets)))
  (set `/Game/Blueprints/UI/HUD.Time` (+ (`/Game/Blueprints/UI/HUD.Time` _ashud) 10) _ashud))

(fn `UserConstructionScript`
  (`parent.UserConstructionScript`))