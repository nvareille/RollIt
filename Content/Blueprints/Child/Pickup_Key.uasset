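; Key pickup Blueprint, a child of a pickup base, that grants the player ball a key.
; Its PickupEffect event increments KeyNb on the first Ball actor found in the world.
; It then finds the first top-level HUD widget and calls DisplayKey with the key count to update the display.
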(event `self.ReceiveBeginPlay`)

(event `self.ReceiveActorBeginOverlap`
  (params (OtherActor :type "Actor Object Reference")))

(event `self.ReceiveTick`
  (params (DeltaSeconds :type "Float (single-precision)"))
  (`parent.ReceiveTick` 0.0))

(event `self.PickupEffect`
  (bind _outactors (`GameplayStatics.GetAllActorsOfClass` "/Game/Blueprints/Pawns/Ball.Ball_C"))
  (bind _result (`/Engine/EditorBlueprintResources/StandardMacros.IncrementInt` (`/Game/Blueprints/Pawns/Ball.KeyNb` (`KismetArrayLibrary.Array_Get` _outactors)))
    (:`  `
      (bind _foundwidgets (`WidgetBlueprintLibrary.GetAllWidgetsOfClass` "/Game/Blueprints/UI/HUD.HUD_C"))
      (bind _ashud (cast `/Game/Blueprints/UI/HUD` (`KismetArrayLibrary.Array_Get` _foundwidgets)))
      (`/Game/Blueprints/UI/HUD.DisplayKey` _ashud _result))))

(fn `UserConstructionScript`
  (`parent.UserConstructionScript`))