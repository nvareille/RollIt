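; One-shot trigger actor that plays an assigned sound through TutoPlayer when an actor overlaps it, while ducking the volume of SoundPlayer.
; The overlap disables the box collision, starts the sound and copies its duration into a countdown.
; Tick holds SoundPlayer at low volume until the countdown expires, then raises it to a fixed level and destroys the trigger.
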(event `self.ReceiveTick`
  (params (DeltaSeconds :type "Float (single-precision)"))
  (bind _audiocomponent (`AmbientSound.AudioComponent` (`self.SoundPlayer`)))
  (if (`self.Action`)
    (bind _output_get (set `self.Duration` (- (`self.Duration`) DeltaSeconds)))
    (if (< _output_get 0.0)
      (`AudioComponent.SetVolumeMultiplier` _audiocomponent 0.35)
      (`self.K2_DestroyActor`)
      (else
        (`AudioComponent.SetVolumeMultiplier` _audiocomponent 0.1)))))

(event `self.ReceiveActorBeginOverlap`
  (params (OtherActor :type "Actor Object Reference"))
  (bind _soundtoplay (`self.SoundToPlay`))
  (bind _audiocomponent (`AmbientSound.AudioComponent` (`self.TutoPlayer`)))
  (set `self.Action` true)
  (`AudioComponent.SetSound` _audiocomponent _soundtoplay)
  (`AudioComponent.Play` _audiocomponent 0.0)
  (`AudioComponent.SetVolumeMultiplier` (`AmbientSound.AudioComponent` (`self.SoundPlayer`)) 0.1)
  (set `self.Duration` (`SoundBase.Duration` _soundtoplay))
  (`PrimitiveComponent.SetCollisionEnabled` (`self.Box`) "NoCollision"))

(fn `UserConstructionScript`)