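; FallCatcher is a trigger actor that catches the ball when it falls, returning it to a respawn point and costing the player a life.
; On overlap it filters actors by a "Ball" display-name prefix, moves the ball to Respawn, and toggles physics simulation off and on, likely to reset its momentum.
; It then calls LoseLife on the HUD widget, found and cached at BeginPlay.
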(event `self.ReceiveBeginPlay`
  (bind _foundwidgets (`WidgetBlueprintLibrary.GetAllWidgetsOfClass` "/Game/Blueprints/UI/HUD.HUD_C"))
  (set `self.HUD` (`KismetArrayLibrary.Array_Get` _foundwidgets)))

(event `self.ReceiveActorBeginOverlap`
  (params (OtherActor :type "Actor Object Reference"))
  (if (`KismetStringLibrary.StartsWith` (`KismetSystemLibrary.GetDisplayName` OtherActor) "Ball")
    (bind _asball (cast `/Game/Blueprints/Pawns/Ball` OtherActor))
    (`self.K2_SetActorLocation` _asball (`self.Respawn`) false false)
    (`PrimitiveComponent.SetSimulatePhysics` (`/Game/Blueprints/Pawns/Ball.Sphere` _asball) false)
    (`PrimitiveComponent.SetSimulatePhysics` (`/Game/Blueprints/Pawns/Ball.Sphere` _asball) true)
    (bind _ashud (cast `/Game/Blueprints/UI/HUD` (`self.HUD`)))
    (`/Game/Blueprints/UI/HUD.LoseLife` _ashud)))

(event `self.ReceiveTick`
  (params (DeltaSeconds :type "Float (single-precision)")))

(fn `UserConstructionScript`)