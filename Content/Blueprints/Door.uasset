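; Key-locked door that opens once when the player's Ball enters its trigger while holding at least one key.
; BeginPlay caches the first Ball actor as the player, and the overlap spends one key, sets IsOn to block repeats, and updates the HUD key display.
; A timeline then slides the door downward by adding a curve-scaled world offset on every update, so the movement accumulates rather than interpolating between fixed positions.
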(event `self.ReceiveBeginPlay`
  ;[1 1 1] Get Player
  (bind _outactors (`GameplayStatics.GetAllActorsOfClass` "/Game/Blueprints/Pawns/Ball.Ball_C"))
  (set `self.Player` (`KismetArrayLibrary.Array_Get` _outactors)))

(event `self.Trigger.OnComponentBeginOverlap`
  (params (OtherActor :type "Actor Object Reference") (OtherComp :type "PrimitiveComponent Object Reference") (OtherBodyIndex :type Integer) (bFromSweep :type Boolean) (SweepResult :type "HitResult Structure (by ref)"))
  (bind _player (`self.Player`))
  (bind _asball (cast `/Game/Blueprints/Pawns/Ball` _player))
  (if (and (and (> (`/Game/Blueprints/Pawns/Ball.KeyNb` _asball) 0) (== OtherActor _player)) (not (`self.IsOn`)))
    (bind _asball_2 (cast `/Game/Blueprints/Pawns/Ball` (`self.Player`)))
    (bind _result (`/Engine/EditorBlueprintResources/StandardMacros.DecrementInt` (`/Game/Blueprints/Pawns/Ball.KeyNb` _asball_2))
      (:`  `
        (set `self.IsOn` true)
        (bind _foundwidgets (`WidgetBlueprintLibrary.GetAllWidgetsOfClass` "/Game/Blueprints/UI/HUD.HUD_C"))
        (bind _ashud (cast `/Game/Blueprints/UI/HUD` (`KismetArrayLibrary.Array_Get` _foundwidgets)))
        (`/Game/Blueprints/UI/HUD.DisplayKey` _ashud _result)
        ;[1 1 1] Animate Opening
        (bind (_direction _movement) (`Timeline|Timeline_Open`)
          (:`Update`
            (`SceneComponent.K2_AddWorldOffset` (`self.Door`) (`KismetMathLibrary.VLerp` (0.0 0.0 0.0) (0.0 0.0 -50.0) _movement) false false)))))))

(fn `UserConstructionScript`)