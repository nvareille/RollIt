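; Player controller that rolls a possessed Ball pawn with torque relative to camera yaw, while look input orbits the camera around the sphere.
; Reversing direction converts accumulated per-axis input into a torque multiplier that decays on Tick, and the Acceleration action doubles torque.
; Brake freezes the ball by disabling physics simulation, then starts a cooldown on release, with a dynamic material colour showing brake state.
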(event `self.ReceiveBeginPlay`
  (bind _asball (cast `/Game/Blueprints/Pawns/Ball` (`self.K2_GetPawn`)))
  (bind _output_get (set `self.BallVar` _asball))
  (bind _sphere (`/Game/Blueprints/Pawns/Ball.Sphere` _output_get))
  (bind _output_get_2 (set `self.Sphere` _sphere))
  (set `self.CameraInstance` (`/Game/Blueprints/Pawns/Ball.Camera` _asball))
  (bind _returnvalue (`KismetMaterialLibrary.CreateDynamicMaterialInstance` _sphere "/Game/Materials/BallMaterial.BallMaterial"))
  (bind _output_get_3 (set `self.Material` _returnvalue))
  (`MaterialInstanceDynamic.SetVectorParameterValue` _output_get_3 "BrakeColor" (struct :`B` 1.0 :`A` 1.0))
  (`PrimitiveComponent.SetMaterial` _output_get_2 0 _output_get_3))

(event `InputAxis|MoveRight`
  (params (AxisValue :type "Float (single-precision)"))
  (bind _xaccel (`self.XAccel`))
  (if (or (and (> AxisValue 0.0) (< _xaccel 0.0)) (and (> _xaccel 0.0) (< AxisValue 0.0)))
    (set `self.XMultiplier` (`KismetMathLibrary.Abs` _xaccel))
    (set `self.XAccel` 0.0)
    (set `self.XBurst` true)
    (else
      (set `self.XAccel` (+ (* AxisValue 0.09) _xaccel))
      (`PrimitiveComponent.AddTorque` (`self.Sphere`) (`KismetMathLibrary.RotateAngleAxis` (`KismetMathLibrary.MakeVector` (+ (* AxisValue -10000.0 (`self.Speed`) (`self.XMultiplier`)) (* 5.0 (`KismetMathLibrary.Conv_BoolToDouble` (`self.XBurst`))))) (.yaw (`SceneComponent.K2_GetComponentRotation` (`self.CameraInstance`))) (0.0 0.0 1.0)) "None" false)
      (set `self.XBurst` false))))

(event `InputAxis|MoveForward`
  (params (AxisValue :type "Float (single-precision)"))
  (bind _yaccel (`self.YAccel`))
  (if (or (and (> AxisValue 0.0) (< _yaccel 0.0)) (and (> _yaccel 0.0) (< AxisValue 0.0)))
    (set `self.YMultiplier` (`KismetMathLibrary.Abs` _yaccel))
    (set `self.YAccel` 0.0)
    (set `self.YBurst` true)
    (else
      (set `self.YAccel` (+ (* AxisValue 0.09) _yaccel))
      (`PrimitiveComponent.AddTorque` (`self.Sphere`) (`KismetMathLibrary.RotateAngleAxis` (`KismetMathLibrary.MakeVector` 0.0 (+ (* AxisValue 10000.0 (`self.Speed`) (`self.YMultiplier`)) (* 5.0 (`KismetMathLibrary.Conv_BoolToDouble` (`self.YBurst`))))) (.yaw (`SceneComponent.K2_GetComponentRotation` (`self.CameraInstance`))) (0.0 0.0 1.0)) "None" false)
      (set `self.YBurst` false))))

(event `InputAxis|LookRight`
  (params (AxisValue :type "Float (single-precision)"))
  (bind _returnvalue (* AxisValue 2.0))
  (bind _camerainstance (`self.CameraInstance`))
  (bind _returnvalue_2 (`SceneComponent.K2_GetComponentLocation` (`self.Sphere`)))
  (`SceneComponent.K2_AddWorldRotation` _camerainstance (`KismetMathLibrary.MakeRotator` 0.0 0.0 _returnvalue) false false)
  (`SceneComponent.K2_SetWorldLocation` _camerainstance (+ (`KismetMathLibrary.RotateAngleAxis` (- (`SceneComponent.K2_GetComponentLocation` (`self.CameraInstance`)) _returnvalue_2) _returnvalue (0.0 0.0 1.0)) _returnvalue_2) false false))

(event `InputAction|Acceleration`
  (params (Key :type "Key Structure" :default "AnyKey"))
  (:`Pressed`
    (set `self.Speed` 2.0))
  (:`Released`
    (set `self.Speed` 1.0)))

(event `InputAction|Brake`
  (params (Key :type "Key Structure" :default "AnyKey"))
  (bind _sphere (`self.Sphere`))
  (bind _returnvalue (<= (`self.BreakCooldown`) 0.0))
  (:`Pressed`
    (if _returnvalue
      (`PrimitiveComponent.SetSimulatePhysics` _sphere false)
      (`MaterialInstanceDynamic.SetVectorParameterValue` (`self.Material`) "BrakeColor" (struct :`R` 1.0 :`A` 1.0))
      (set `self.BrakeAction` true)))
  (:`Released`
    (if _returnvalue
      (`PrimitiveComponent.SetSimulatePhysics` _sphere true)
      (set `self.BreakCooldown` 2.0)
      (set `self.BrakeAction` false))))

(event `self.ReceiveTick`
  (params (DeltaSeconds :type "Float (single-precision)"))
  (bind _xmultiplier (`self.XMultiplier`))
  (bind _ymultiplier (`self.YMultiplier`))
  (if (`KismetMathLibrary.BooleanNAND` (> DeltaSeconds 0.0) (`self.BrakeAction`))
    (bind _output_get (set `self.BreakCooldown` (- (`self.BreakCooldown`) DeltaSeconds)))
    (if (< _output_get 0.0)
      (`MaterialInstanceDynamic.SetVectorParameterValue` (`self.Material`) "BrakeColor" (struct :`A` 1.0))))
  (if (> _xmultiplier 1.0)
    (bind _output_get_2 (set `self.XMultiplier` (* _xmultiplier 0.8))))
  (if (< _output_get_2 1.0)
    (set `self.XMultiplier` 1.0))
  (if (> _ymultiplier 1.0)
    (bind _output_get_3 (set `self.YMultiplier` (* _ymultiplier 0.8))))
  (if (< _output_get_3 1.0)
    (set `self.YMultiplier` 1.0))
  (`KismetSystemLibrary.PrintString` (`KismetStringLibrary.Conv_DoubleToString` (`self.YMultiplier`)))
  (`KismetSystemLibrary.PrintString` (`KismetStringLibrary.Conv_DoubleToString` (`self.XMultiplier`))))

(fn `UserConstructionScript`
  (set `self.Speed` 1.0)
  (set `self.Brake` 1.0)
  (set `self.XMultiplier` 1.0)
  (set `self.YMultiplier` 1.0))